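; Spawner that lays a random-length strip of ground tiles at game start, beginning beneath the player pawn.
; Each tile class is picked randomly from GroundToSpawn, placed at the previous tile's SpawnPoint and given a reference to the spawner.
; Per-type grass, highway, river and track functions are not run from BeginPlay; river and track ones spawn BP_Grass.
; Object-spawn helpers place random ObjectSpawns actors at the spawner's transform.
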(event EventBeginPlay
  (CallFunction|SpawnInitialGround))

(fn ConstructionScript)

(fn SpawnGrass
  (params (SpawnLocation :type Vector :default "0,0,0.000000"))
  (bind _returnvalue (Game|SpawnActorfromClass "/Game/BluePrints/OldFloor/BP_Grass.BP_Grass_C" (Math|Transform|MakeTransform SpawnLocation "0, 0, 0" "1,1,1") "Undefined" 0 0))
  (bind _output_get (Variables|Default|SetNewestGrass _returnvalue))
  (Variables|/Game/BluePrints/OldFloor/BP_Grass.BP_Grass_C|SetGrassSpawner _output_get self))

(fn SpawnGrassatSpawnPoint
  (CallFunction|SpawnGrass (Transformation|GetWorldLocation (Variables|/Game/BluePrints/OldFloor/BP_Grass.BP_Grass_C|GetSpawnPoint (Variables|Default|GetNewestGrass)))))

(fn SpawnInitialGrass
  (for _index (range 0 (Math|Random|RandomIntegerinRange 0 18))
    (Utilities|IsValid (Variables|Default|GetNewestGrass)
      (:Is%20Valid
        (CallFunction|SpawnGrassatSpawnPoint))
      (:Is%20Not%20Valid
        (CallFunction|SpawnGrass (- (Transformation|GetActorLocation (Game|Player|GetPlayerPawn 0)) "0, 0,120.000000"))))))

(fn SpawnInitialHighWay
  (for _index (range 0 (Math|Random|RandomIntegerinRange 0 18))
    (Utilities|IsValid (Variables|Default|GetNewestHighway)
      (:Is%20Valid
        (CallFunction|SpawnInitialHighWay))
      (:Is%20Not%20Valid
        (CallFunction|SpawnHighway (- (Transformation|GetActorLocation (Game|Player|GetPlayerPawn 0)) "0, 0,120.000000"))))))

(fn SpawnHighway
  (params (SpawnLocation :type Vector :default "0,0,0.000000"))
  (bind _returnvalue (Game|SpawnActorfromClass "/Game/BluePrints/OldFloor/BP_Highway.BP_Highway_C" (Math|Transform|MakeTransform SpawnLocation "0, 0, 0" "1,1,1") "Undefined" 0 0))
  (bind _output_get (Variables|Default|SetNewestHighway _returnvalue))
  (Variables|/Game/BluePrints/OldFloor/BP_Grass.BP_Grass_C|SetGrassSpawner _output_get self))

(fn SpawnInitialRiver
  (for _index (range 0 (Math|Random|RandomIntegerinRange 0 18))
    (Utilities|IsValid (Variables|Default|GetNewestRiver)
      (:Is%20Valid
        (CallFunction|SpawnRiveratSpawnPoint))
      (:Is%20Not%20Valid
        (CallFunction|SpawnRiver (- (Transformation|GetActorLocation (Game|Player|GetPlayerPawn 0)) "0, 0,120.000000"))))))

(fn SpawnInitialTracks
  (for _index (range 0 (Math|Random|RandomIntegerinRange 0 18))
    (Utilities|IsValid (Variables|Default|GetNewestTracks)
      (:Is%20Valid
        (CallFunction|SpawnTracksatSpawnPoint))
      (:Is%20Not%20Valid
        (CallFunction|SpawnTracks (- (Transformation|GetActorLocation (Game|Player|GetPlayerPawn 0)) "0, 0,120.000000"))))))

(fn SpawnRiver
  (params (SpawnLocation :type Vector :default "0,0,0.000000"))
  (bind _returnvalue (Game|SpawnActorfromClass "/Game/BluePrints/OldFloor/BP_Grass.BP_Grass_C" (Math|Transform|MakeTransform SpawnLocation "0, 0, 0" "1,1,1") "Undefined" 0 0))
  (bind _output_get (Variables|Default|SetNewestGrass _returnvalue))
  (Variables|/Game/BluePrints/OldFloor/BP_Grass.BP_Grass_C|SetGrassSpawner _output_get self))

(fn SpawnTracks
  (params (SpawnLocation :type Vector :default "0,0,0.000000"))
  (bind _returnvalue (Game|SpawnActorfromClass "/Game/BluePrints/OldFloor/BP_Grass.BP_Grass_C" (Math|Transform|MakeTransform SpawnLocation "0, 0, 0" "1,1,1") "Undefined" 0 0))
  (bind _output_get (Variables|Default|SetNewestGrass _returnvalue))
  (Variables|/Game/BluePrints/OldFloor/BP_Grass.BP_Grass_C|SetGrassSpawner _output_get self))

(fn SpawnHighwayatSpawnPoint
  (CallFunction|SpawnHighway (Transformation|GetWorldLocation (Variables|/Game/BluePrints/OldFloor/BP_Grass.BP_Grass_C|GetSpawnPoint (Variables|Default|GetNewestHighway)))))

(fn SpawnRiveratSpawnPoint
  (CallFunction|SpawnRiver (Transformation|GetWorldLocation (Variables|/Game/BluePrints/OldFloor/BP_Grass.BP_Grass_C|GetSpawnPoint (Variables|Default|GetNewestRiver)))))

(fn SpawnTracksatSpawnPoint
  (CallFunction|SpawnTracks (Transformation|GetWorldLocation (Variables|/Game/BluePrints/OldFloor/BP_Grass.BP_Grass_C|GetSpawnPoint (Variables|Default|GetNewestTracks)))))

(fn SpawnGround
  (params (SpawnLocation :type Vector :default "0.000000,0,0.000000"))
  (bind _returnvalue (Game|SpawnActorfromClass (Utilities|Array|Get(acopy) (Variables|Default|GetGroundToSpawn) (Math|Random|RandomIntegerinRange 0 3)) (Math|Transform|MakeTransform SpawnLocation "0, 0, 0" "1,1,1") "Undefined" 0 0))
  (bind _output_get (Variables|Default|SetLastestGround _returnvalue))
  (Variables|/Game/BluePrints/BP_BaseFloor.BP_BaseFloor_C|SetGroundSpawner _output_get self))

(fn SpawnGroundatSpawnPoint
  (CallFunction|SpawnGround (Transformation|GetWorldLocation (Variables|/Game/BluePrints/BP_BaseFloor.BP_BaseFloor_C|GetSpawnPoint (Variables|Default|GetLastestGround)))))

(fn SpawnInitialGround
  (for _index (range 0 (Math|Random|RandomIntegerinRange 0 18))
    (Utilities|IsValid (Variables|Default|GetLastestGround)
      (:Is%20Valid
        (CallFunction|SpawnGroundatSpawnPoint))
      (:Is%20Not%20Valid
        (CallFunction|SpawnGround (- (Transformation|GetActorLocation (Game|Player|GetPlayerPawn 0)) "0.000000, 0,120.000000"))))))

(fn SpawnGrassObject
  (Game|SpawnActorfromClass (Utilities|Array|Get(acopy) (Variables|Default|GetObjectSpawns) (Math|Random|RandomIntegerinRange 0 6)) (Math|Transform|MakeTransform (Transformation|GetActorLocation) (Transformation|GetActorRotation)) "Undefined" 0 0))

(fn SpawnObject
  (bind _returnvalue (Game|SpawnActorfromClass (Utilities|Array|Get(acopy) (Variables|Default|GetObjectSpawns) (Math|Random|RandomIntegerinRange 0 (- (Utilities|Array|Length (Variables|Default|GetObjectSpawns)) 1))) (Math|Transform|MakeTransform (Transformation|GetActorLocation) (Transformation|GetActorRotation)) "AdjustIfPossibleButAlwaysSpawn" 0 0))
  (Variables|Default|SetCurrentObject _returnvalue))