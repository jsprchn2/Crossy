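; GrassFloor is a floor actor that provides a grass-covered surface in the level.
; Its construction script runs the parent's, then adds a static mesh component at a fixed relative offset and applies the Grass_MT material to it.
; SpawnObjects is empty: its logic to spawn a random rock, tree or ObjectsToSpawn class at the actor's transform is disconnected and never runs.
; The event graph holds only disabled or empty events.
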(event OnComponentWake(StaticMesh)
  (params (WakingComponent :type Primitive%20Component%20Object%20Reference) (BoneName :type Name :default "None")))

(event EventBeginPlay
  (|CallParentFunction) ; This node is disabled and will not be called.\nDrag off pins to build functionality.
)

(event Collision|EventActorBeginOverlap
  (params (OtherActor :type Actor%20Object%20Reference))
  (|CallParentFunction OtherActor) ; This node is disabled and will not be called.\nDrag off pins to build functionality.
)

(event EventTick
  (params (DeltaSeconds :type Float%20%28single-precision%29))
  (|CallParentFunction DeltaSeconds) ; This node is disabled and will not be called.\nDrag off pins to build functionality.
)

(fn ConstructionScript
  (|CallParentFunction)
  (AddComponent|AddStaticMeshComponent false (Math|Conversions|ToTransform(Vector) (Math|Vector|MakeVector -2e+02 -2e+02 19.0)))
  (Rendering|Material|SetMaterial (Variables|Default|GetStaticMeshComponent) 0 "/Game/Materials/grass.grass_MT"))

(fn SpawnObjects)