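; Floor Blueprint that blinks two lights, Light1 and Light2, after play begins.
; BeginPlay starts a timeline whose Update pin serves only as a repeating trigger for half-second Delays, with no track values used.
; Each elapsed Delay toggles Light1's visibility, then a second Delay toggles Light2 half a second later, staggering the blink while the timeline runs.
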(event EventBeginPlay
  (|CallParentFunction)
  (Timeline|Timeline_0 Play
    (:Update
      (Utilities|FlowControl|Delay 0.5)
      (Utilities|FlowControl|Sequence
        (:then_0
          (Rendering|ToggleVisibility (Variables|Default|GetLight1) false))
        (:then_1
          (Utilities|FlowControl|Delay 0.5)
          (Rendering|ToggleVisibility (Variables|Default|GetLight2) false))))))

(event Collision|EventActorBeginOverlap
  (params (OtherActor :type Actor%20Object%20Reference))
  (|CallParentFunction OtherActor) ; This node is disabled and will not be called.\nDrag off pins to build functionality.
)

(event EventTick
  (params (DeltaSeconds :type Float%20%28single-precision%29))
  (|CallParentFunction DeltaSeconds) ; This node is disabled and will not be called.\nDrag off pins to build functionality.
)

(fn ConstructionScript
  (|CallParentFunction))