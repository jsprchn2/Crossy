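; Player-controlled chicken character that hops in steps on the W, A, S and D keys.
; Each key release jumps, plays a hop sound, turns the mesh to face that way and moves the actor by a swept MaxSpd offset.
; Mesh overlaps only print debug text, and the movement axis events are unwired.
; Reset and ChickenDied restart the player at a player start, though nothing here calls them.
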(event OnComponentBeginOverlap(StaticMesh)
  (params (OverlappedComponent :type Primitive%20Component%20Object%20Reference) (OtherActor :type Actor%20Object%20Reference) (OtherComp :type Primitive%20Component%20Object%20Reference) (OtherBodyIndex :type Integer) (bFromSweep :type Boolean) (SweepResult :type Hit%20Result%20Structure%20%28by%20ref%29))
  (Development|PrintString (Utilities|GetDisplayName self))
  (Development|PrintString "Hello")
  (Development|PrintString (Utilities|GetDisplayName OtherActor)))

(event EventBeginPlay)

(event Collision|EventActorBeginOverlap
  (params (OtherActor :type Actor%20Object%20Reference)))

(event EventTick
  (params (DeltaSeconds :type Float%20%28single-precision%29))
  (bind _returnvalue (Class|Pawn|ConsumeMovementInputVector))
  (Transformation|AddActorLocalOffset (* _returnvalue DeltaSeconds) true false))

(event Input|AxisEvents|InputAxismoveforward
  (params (AxisValue :type Float%20%28single-precision%29)))

(event Input|AxisEvents|InputAxismoveright
  (params (AxisValue :type Float%20%28single-precision%29)))

(event Input|KeyboardEvents|W
  (params (Key :type Key%20Structure))
  (:Pressed
    (Character|StopJumping))
  (:Released
    (Character|Jump)
    (Audio|PlaySound2D "/Game/BluePrints/Sounds/hop2b.hop2b" 1.0 1.0 0.0 0 0)
    (Transformation|SetRelativeRotation (Variables|Default|GetStaticMesh) "0,90.000000, 0" false false)
    (Transformation|AddActorWorldOffset (* (Transformation|GetActorForwardVector) (Variables|Default|GetMaxSpd)) true)
    (Utilities|FlowControl|Delay 1.0)
    (Variables|Default|SetCurrentlyJumping true)))

(event Input|KeyboardEvents|S
  (params (Key :type Key%20Structure))
  (:Pressed
    (Character|StopJumping))
  (:Released
    (Character|Jump)
    (Audio|PlaySound2D "/Game/BluePrints/Sounds/hop2b.hop2b" 1.0 1.0 0.0 0 0)
    (Transformation|SetRelativeRotation (Variables|Default|GetStaticMesh) "0,270.000000, 0" false false)
    (Transformation|AddActorWorldOffset (* (* (Transformation|GetActorForwardVector) (Variables|Default|GetMaxSpd)) -1.0) true)
    (Variables|Default|SetCurrentlyJumping true)))

(event Input|KeyboardEvents|D
  (params (Key :type Key%20Structure))
  (:Pressed
    (Character|StopJumping))
  (:Released
    (Character|Jump)
    (Audio|PlaySound2D "/Game/BluePrints/Sounds/hop2b.hop2b" 1.0 1.0 0.0 0 0)
    (Transformation|SetRelativeRotation (Variables|Default|GetStaticMesh) "0,180.000000, 0" false false)
    (Transformation|AddActorWorldOffset (* (Transformation|GetActorRightVector) (Variables|Default|GetMaxSpd)) true)
    (Variables|Default|SetCurrentlyJumping true)))

(event Input|KeyboardEvents|A
  (params (Key :type Key%20Structure))
  (:Pressed
    (Character|StopJumping))
  (:Released
    (Character|Jump)
    (Audio|PlaySound2D "/Game/BluePrints/Sounds/hop2b.hop2b" 1.0 1.0 0.0 0 0)
    (Transformation|SetRelativeRotation (Variables|Default|GetStaticMesh) "0, 0, 0" false false)
    (Transformation|AddActorWorldOffset (* (* (Transformation|GetActorRightVector) (Variables|Default|GetMaxSpd)) -1.0) true)
    (Variables|Default|SetCurrentlyJumping true)))

(fn ConstructionScript)

(fn Reset
  (if (Variables|Default|GetDead)
    (Class|GameModeBase|RestartPlayeratPlayerStart (Variables|Default|GetGameMode) (Game|GetPlayerController 0))))

(fn ChickenDied
  (Variables|Default|SetDead false)
  (Class|GameModeBase|RestartPlayeratPlayerStart (Variables|Default|GetGameMode)))