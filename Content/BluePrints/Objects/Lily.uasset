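; Lily is an object actor that can travel along a track's spline and plays a splash sound when hit.
; When Move is set, BeginPlay starts the ObjectMove timeline, with play rate set by Duration and start time by MoveOffset.
; Each update maps the timeline alpha to a spline distance on TrackRef and applies that world location and rotation.
; Box hits play the 2D sound, while its overlap event does nothing.
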(event OnComponentBeginOverlap(Box)
  (params (OverlappedComponent :type Primitive%20Component%20Object%20Reference) (OtherActor :type Actor%20Object%20Reference) (OtherComp :type Primitive%20Component%20Object%20Reference) (OtherBodyIndex :type Integer) (bFromSweep :type Boolean) (SweepResult :type Hit%20Result%20Structure%20%28by%20ref%29)))

(event OnComponentHit(Box)
  (params (HitComponent :type Primitive%20Component%20Object%20Reference) (OtherActor :type Actor%20Object%20Reference) (OtherComp :type Primitive%20Component%20Object%20Reference) (NormalImpulse :type Vector :default "0, 0, 0") (Hit :type Hit%20Result%20Structure%20%28by%20ref%29))
  (Audio|PlaySound2D "/Game/BluePrints/Sounds/lilysplash.lilysplash" 1.0 1.0 0.0 0 0))

(event Custom|MoveLily
  (Components|Timeline|SetPlayRate (Variables|Default|GetObjectMove) (/ 1.0 (Variables|Default|GetDuration)))
  (Components|Timeline|SetNewTime (Variables|Default|GetObjectMove) (Variables|Default|GetMoveOffset))
  (bind _alpha (Timeline|ObjectMove Play)
    (:Update
      (Variables|Default|SetAlpha _alpha)
      (Transformation|SetActorLocationAndRotation (Spline|GetLocationatDistanceAlongSpline (Variables|/Game/BluePrints/SpawnTrack.SpawnTrack_C|GetSpline (Variables|Default|GetTrackRef)) (Math|Float|Lerp 0.0 (Spline|GetSplineLength (Variables|/Game/BluePrints/SpawnTrack.SpawnTrack_C|GetSpline (Variables|Default|GetTrackRef))) (Variables|Default|GetAlpha)) "World") (Spline|GetRotationatDistanceAlongSpline (Variables|/Game/BluePrints/SpawnTrack.SpawnTrack_C|GetSpline (Variables|Default|GetTrackRef)) (Math|Float|Lerp 0.0 (Spline|GetSplineLength (Variables|/Game/BluePrints/SpawnTrack.SpawnTrack_C|GetSpline (Variables|Default|GetTrackRef))) (Variables|Default|GetAlpha)) "World")))))

(event EventBeginPlay
  (if (Variables|Default|GetMove)
    (CallFunction|MoveLily)))

(fn ConstructionScript
  (|CallParentFunction))