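; Car23 is a vehicle Blueprint that drives itself along the spline of a referenced track actor.
; On BeginPlay, if Move is set, it plays the CarMove timeline with play rate derived from Duration and a configurable start offset.
; Each update maps the timeline alpha to distance along the spline and sets the car's world location and rotation to match.
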(event Custom|MoveCar
  (Components|Timeline|SetPlayRate (Variables|Default|GetCarMove) (/ 1.0 (Variables|Default|GetDuration)))
  (Components|Timeline|SetNewTime (Variables|Default|GetCarMove) (Variables|Default|GetCarMoveOffset))
  (bind _alpha (Timeline|CarMove Play)
    (:Update
      (Variables|Default|SetAlpha _alpha)
      (Transformation|SetActorLocationAndRotation (Spline|GetLocationatDistanceAlongSpline (Variables|/Game/BluePrints/SpawnTrack.SpawnTrack_C|GetSpline (Variables|Default|GetTrackRef)) (Math|Float|Lerp 0.0 (Spline|GetSplineLength (Variables|/Game/BluePrints/SpawnTrack.SpawnTrack_C|GetSpline (Variables|Default|GetTrackRef))) (Variables|Default|GetAlpha)) "World") (Spline|GetRotationatDistanceAlongSpline (Variables|/Game/BluePrints/SpawnTrack.SpawnTrack_C|GetSpline (Variables|Default|GetTrackRef)) (Math|Float|Lerp 0.0 (Spline|GetSplineLength (Variables|/Game/BluePrints/SpawnTrack.SpawnTrack_C|GetSpline (Variables|Default|GetTrackRef))) (Variables|Default|GetAlpha)) "World")))))

(event EventBeginPlay
  (if (Variables|Default|GetMove)
    (CallFunction|MoveCar)))

(fn ConstructionScript)