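; Car22 is a vehicle actor that drives along a track's spline and kills the Chicken player on contact.
; On BeginPlay, if Move is set, the CarMove timeline starts from an offset, with its play rate scaled by Duration.
; Its alpha maps to distance along TrackRef's spline, setting world location and rotation.
; A Box overlap with a Chicken marks it dead and asks GM to restart the player.
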(event OnComponentBeginOverlap(Box)
  (params (OverlappedComponent :type Primitive%20Component%20Object%20Reference) (OtherActor :type Actor%20Object%20Reference) (OtherComp :type Primitive%20Component%20Object%20Reference) (OtherBodyIndex :type Integer) (bFromSweep :type Boolean) (SweepResult :type Hit%20Result%20Structure%20%28by%20ref%29))
  (bind _aschicken (Utilities|Casting|CastToChicken OtherActor))
  (Variables|/Game/BluePrints/Game/Chicken.Chicken_C|SetDead _aschicken true)
  (Class|GameModeBase|RestartPlayer (Variables|Default|GetGM)))

(event Custom|MoveCar
  (Components|Timeline|SetPlayRate (Variables|Default|GetCarMove) (/ 1.0 (Variables|Default|GetDuration)))
  (Components|Timeline|SetNewTime (Variables|Default|GetCarMove) (Variables|Default|GetCarMoveOffset))
  (bind _alpha (Timeline|CarMove Play)
    (:Update
      (Variables|Default|SetAlpha _alpha)
      (Transformation|SetActorLocationAndRotation (Spline|GetLocationatDistanceAlongSpline (Variables|/Game/BluePrints/SpawnTrack.SpawnTrack_C|GetSpline (Variables|Default|GetTrackRef)) (Math|Float|Lerp 0.0 (Spline|GetSplineLength (Variables|/Game/BluePrints/SpawnTrack.SpawnTrack_C|GetSpline (Variables|Default|GetTrackRef))) (Variables|Default|GetAlpha)) "World") (Spline|GetRotationatDistanceAlongSpline (Variables|/Game/BluePrints/SpawnTrack.SpawnTrack_C|GetSpline (Variables|Default|GetTrackRef)) (Math|Float|Lerp 0.0 (Spline|GetSplineLength (Variables|/Game/BluePrints/SpawnTrack.SpawnTrack_C|GetSpline (Variables|Default|GetTrackRef))) (Variables|Default|GetAlpha)) "World")))))

(event EventBeginPlay
  (if (Variables|Default|GetMove)
    (CallFunction|MoveCar)))

(fn ConstructionScript)

(fn SpawnVehicle)